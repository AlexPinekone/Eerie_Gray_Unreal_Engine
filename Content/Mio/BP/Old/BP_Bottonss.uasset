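; BP_Bottonss is a floor-trigger button that opens a door once the player's pickup count matches a required amount.
; On overlap it compares BP_FP's PickUpPlayer to LimitCollectDoors for exact equality.
; A match fires once through DoOnce, lowering the button mesh, switching it to the Rojo material and destroying the linked Door.
; Otherwise it prints a Spanish "need to access" message that inserts the player's current count rather than the limit.
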(event EventBeginPlay)

(event Collision|EventActorBeginOverlap
  (params (OtherActor :type Actor%20Object%20Reference))
  (bind _returnvalue (Game|GetPlayerCharacter 0))
  (bind _asbp_fp (Utilities|Casting|CastToBP_FP _returnvalue))
  (bind _pickupplayer (Variables|/Game/Mio/BP/BP_FP.BP_FP_C|GetPickUpPlayer _asbp_fp))
  (if (== (Variables|Default|GetLimit%20Collect%20Doors) _pickupplayer)
    (Utilities|FlowControl|DoOnce false
      (:Completed
        (Transformation|AddLocalOffset (Variables|Default|GetButton) "0, 0,-90.000000" false false)
        (Rendering|Material|SetMaterial (Variables|Default|GetButton) 0 "/Game/Mio/Material/Rojo.Rojo")
        (Actor|DestroyActor (Variables|MP|GetDoor))))
    (else
      (Development|PrintString (Utilities|String|Append "Necesitas" (Utilities|String|ToString(Integer) _pickupplayer) " para acceder") true true "(R=1.000000,G=0.096132,B=0.000000,A=1.000000)" 3.0))))

(event EventTick
  (params (DeltaSeconds :type Float%20%28single-precision%29)))

(fn ConstructionScript)