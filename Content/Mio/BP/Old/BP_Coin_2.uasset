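; BP_Coin_2 is a coin pickup Actor that reacts when the first player character overlaps it.
; The overlap stores the coin's location and plays a collect timeline, which hides the coin when finished and plays a sound once at the player's location.
; Each timeline update sets the coin's location to world origin, as the Lerp from start location to player is left unconnected.
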(event EventBeginPlay)

(event Collision|EventActorBeginOverlap
  (params (OtherActor :type Actor%20Object%20Reference))
  (if (== OtherActor (Game|GetPlayerCharacter 0))
    (Variables|Default|SetStart%20Location (Transformation|GetActorLocation))
    (bind _move (Timeline|Colect%20Timeline Play)
      (:Update
        ;[1 1 1] Posicion
        (Transformation|SetActorLocation "0, 0, 0" false false))
      (:Finished
        (Rendering|SetActorHiddenInGame true)
        (Utilities|FlowControl|DoOnce false
          (:Completed
            (Audio|SpawnSoundatLocation (Variables|MP|GetSound) (Transformation|GetActorLocation (Game|GetPlayerCharacter 0)) "0, 0, 0" 1.0 1.0 0.0 0 0)))))))

(event EventTick
  (params (DeltaSeconds :type Float%20%28single-precision%29)))

(fn ConstructionScript)