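; BP_OjoBoton is an eye-shaped button that moves its linked Door when first overlapped.
; Nested timelines slide the two eyelids and apply a meat material, calling MuevePuerta from the second timeline's update.
; When LimitCollectDoors is zero or less, it also starts the WJuego widget's count and plays a sound once at the player.
; A pickup-requirement message branch is present but unconnected.
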(event EventBeginPlay)

(event Collision|EventActorBeginOverlap
  (params (OtherActor :type Actor%20Object%20Reference))
  (Utilities|FlowControl|DoOnce false
    (:Completed
      (bind (_direction _x _y) (Timeline|Parpado1A Play)
        (:Update
          (Transformation|SetRelativeLocation (Variables|Default|GetParpado%201) (Math|Vector|MakeVector _x 0.0 _y) false false)
          (bind (_direction_2 _x_2 _y_2) (Timeline|Parpado2A Play)
            (:Update
              (Transformation|SetRelativeLocation (Variables|Default|GetParpado%202) (Math|Vector|MakeVector _x_2 0.0 _y_2) false false)
              (Rendering|Material|SetMaterial (Variables|Default|GetParpado%201) 0 "/Game/Mio/Material/Carne/BP_Meat_01.BP_Meat_01")
              (Rendering|Material|SetMaterial (Variables|Default|GetParpado%202) 0 "/Game/Mio/Material/Carne/BP_Meat_01.BP_Meat_01")
              (if (<= (Variables|Default|GetLimit%20Collect%20Doors) 0)
                (Default|StartCount (Variables|/Game/Mio/BP/BP_FP.BP_FP_C|GetW_Juego (.AsBP%20FP (Utilities|Casting|CastToBP_FP (Game|Player|GetPlayerPawn 0)))))
                (Default|MuevePuerta (Variables|MP|GetDoor))
                (Utilities|FlowControl|DoOnce false
                  (:Completed
                    (Audio|SpawnSoundatLocation (Variables|Default|GetSound) (Transformation|GetActorLocation (Game|GetPlayerCharacter 0)) "0, 0, 0" 1.0 1.0 0.0 0 0)))
                (else
                  (Default|MuevePuerta (Variables|MP|GetDoor)))))))))))

(event EventTick
  (params (DeltaSeconds :type Float%20%28single-precision%29)))

(fn ConstructionScript)