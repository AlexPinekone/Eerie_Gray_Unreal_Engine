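; BP_WeNeedToGo is an end-of-level trigger that marks the player's run as finished and then restarts the level.
; Any overlap on its Box, with no check on the overlapping actor, sets Finalizo on the player's BP_FP.
; It also sets TodasLasCalaberas (all skulls) by whether the player's pickup count equals the total.
; After a fixed delay, it reopens the current level by name.
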(event OnComponentBeginOverlap(Box)
  (params (OverlappedComponent :type Primitive%20Component%20Object%20Reference) (OtherActor :type Actor%20Object%20Reference) (OtherComp :type Primitive%20Component%20Object%20Reference) (OtherBodyIndex :type Integer) (bFromSweep :type Boolean) (SweepResult :type Hit%20Result%20Structure%20%28by%20ref%29))
  (bind _returnvalue (Game|GetPlayerCharacter 0))
  (bind _asbp_fp (Utilities|Casting|CastToBP_FP _returnvalue))
  (Variables|/Game/Mio/BP/BP_FP.BP_FP_C|Setfinalizo _asbp_fp true)
  (if (== (Variables|/Game/Mio/BP/BP_FP.BP_FP_C|GetPickUpsPlayer _asbp_fp) (Variables|/Game/Mio/BP/BP_FP.BP_FP_C|GetPickUpsTotales _asbp_fp))
    (Variables|/Game/Mio/BP/BP_FP.BP_FP_C|SettodasLasCalaberas _asbp_fp true)
    (else
      (Variables|/Game/Mio/BP/BP_FP.BP_FP_C|SettodasLasCalaberas _asbp_fp false)))
  (Utilities|FlowControl|Delay 8.0)
  (bind _returnvalue_2 (Game|GetCurrentLevelName true))
  (Game|OpenLevel(byName) (Utilities|String|StringToName _returnvalue_2)))

(event EventBeginPlay)

(event Collision|EventActorBeginOverlap
  (params (OtherActor :type Actor%20Object%20Reference)))

(event EventTick
  (params (DeltaSeconds :type Float%20%28single-precision%29)))

(fn ConstructionScript)