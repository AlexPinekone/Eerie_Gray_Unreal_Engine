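; BP_WeNeedToGoDeeper is a box trigger that changes the level based on the player's pickup progress.
; Any overlap with the box compares the BP_FP player's PickUpsPlayer count to PickUpsTotales, without checking which actor entered.
; When they match, it destroys every BP_Monstruo in the world; otherwise, it hides the actors in its Gatos array.
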(event OnComponentBeginOverlap(Box)
  (params (OverlappedComponent :type Primitive%20Component%20Object%20Reference) (OtherActor :type Actor%20Object%20Reference) (OtherComp :type Primitive%20Component%20Object%20Reference) (OtherBodyIndex :type Integer) (bFromSweep :type Boolean) (SweepResult :type Hit%20Result%20Structure%20%28by%20ref%29))
  (bind _returnvalue (Game|GetPlayerCharacter 0))
  (bind _asbp_fp (Utilities|Casting|CastToBP_FP _returnvalue))
  (if (== (Variables|/Game/Mio/BP/BP_FP.BP_FP_C|GetPickUpsPlayer _asbp_fp) (Variables|/Game/Mio/BP/BP_FP.BP_FP_C|GetPickUpsTotales _asbp_fp))
    (bind _outactors (Actor|GetAllActorsOfClass "/Game/Mio/BP/BP_Monstruo.BP_Monstruo_C"))
    (for _array_element _outactors
      (Actor|DestroyActor _array_element))
    (else
      (for _array_element_2 (Variables|MP|GetGatos)
        (Rendering|SetActorHiddenInGame _array_element_2 true)))))

(event EventBeginPlay)

(event Collision|EventActorBeginOverlap
  (params (OtherActor :type Actor%20Object%20Reference)))

(event EventTick
  (params (DeltaSeconds :type Float%20%28single-precision%29)))

(fn ConstructionScript)