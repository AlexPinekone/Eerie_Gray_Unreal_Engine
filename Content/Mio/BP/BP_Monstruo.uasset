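; BP_Monstruo is a monster hazard with an animated mouth that restarts the current level when the player touches it.
; On BeginPlay, the BocaArriba timeline offsets the upper and lower mouth meshes from their stored world start locations.
; When the BP_FP player character overlaps the Box, the camera fades to dark red, then the level reloads after the fade duration.
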(event OnComponentBeginOverlap(Box)
  (params (OverlappedComponent :type Primitive%20Component%20Object%20Reference) (OtherActor :type Actor%20Object%20Reference) (OtherComp :type Primitive%20Component%20Object%20Reference) (OtherBodyIndex :type Integer) (bFromSweep :type Boolean) (SweepResult :type Hit%20Result%20Structure%20%28by%20ref%29))
  ;[1 1 1] Colision
  (if (== OtherActor (.AsBP%20FP (Utilities|Casting|CastToBP_FP (Game|GetPlayerCharacter 0))))
    (CameraFades|StartCameraFade (Game|GetPlayerCameraManager 0) 0.0 1.0 (Variables|Default|GetDuration) "(R=0.072917,G=0.000000,B=0.000000,A=1.000000)" false true)
    (Utilities|FlowControl|Delay (Variables|Default|GetDuration))
    (bind _returnvalue (Game|GetCurrentLevelName true))
    (Game|OpenLevel(byName) (Utilities|String|StringToName _returnvalue))))

(event EventBeginPlay
  (Variables|Default|SetInicialLocationBArr (Transformation|GetWorldLocation (Variables|Default|GetBocaArribaMesh)))
  (Variables|Default|SetInicialLocationBAb (Transformation|GetWorldLocation (Variables|Default|GetBocaAbajoMesh)))
  (bind (_direction _barr _bab) (Timeline|BocaArriba Play)
    (:Update
      (Transformation|SetWorldLocation (Variables|Default|GetBocaArribaMesh) (+ (Variables|Default|GetInicialLocationBArr) _barr) false false)
      (Transformation|SetWorldLocation (Variables|Default|GetBocaAbajoMesh) (+ (Variables|Default|GetInicialLocationBAb) _bab) false false))))

(event Collision|EventActorBeginOverlap
  (params (OtherActor :type Actor%20Object%20Reference)))

(event EventTick
  (params (DeltaSeconds :type Float%20%28single-precision%29)))

(fn ConstructionScript)