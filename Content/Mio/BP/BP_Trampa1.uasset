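; BP_Trampa1 is a trap actor ("trampa") that moves along a timeline-driven offset from where it was placed.
; On BeginPlay it stores its location in IniciaLocal and plays the MoveVertica timeline, which sets the actor to that start location plus the track value on each update, without sweep.
; The graphs contain no overlap, damage or tick logic.
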(event EventBeginPlay
  (|CallParentFunction)
  (Variables|Default|SetIniciaLocal (Transformation|GetActorLocation))
  (bind _a (Timeline|MoveVertica Play)
    (:Update
      (Transformation|SetActorLocation (+ (Variables|Default|GetIniciaLocal) _a) false false))))

(event Collision|EventActorBeginOverlap
  (params (OtherActor :type Actor%20Object%20Reference))
  (|CallParentFunction OtherActor) ; This node is disabled and will not be called.\nDrag off pins to build functionality.
)

(event EventTick
  (params (DeltaSeconds :type Float%20%28single-precision%29))
  (|CallParentFunction DeltaSeconds) ; This node is disabled and will not be called.\nDrag off pins to build functionality.
)

(fn ConstructionScript
  (|CallParentFunction))