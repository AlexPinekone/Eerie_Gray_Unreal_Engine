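; BP_Collect is a collectible actor that the player picks up by touching it.
; Overlap with the player character starts the Rotar timeline, which drives the actor's yaw, then hides the actor when finished rather than destroying it.
; A DoOnce on the timeline update triggers, after a short delay, a sound at the player's location and the PickUp call on BP_FP.
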(event EventBeginPlay)

(event Collision|EventActorBeginOverlap
  (params (OtherActor :type Actor%20Object%20Reference))
  (if (== OtherActor (Game|GetPlayerCharacter 0))
    (Variables|Default|SetStartLocation (Transformation|GetActorLocation))
    (bind _move (Timeline|Rotar Play)
      (:Update
        (Transformation|SetActorRotation (Math|Rotator|MakeRotator 0.0 0.0 _move))
        (Utilities|FlowControl|DoOnce false
          (:Completed
            (Utilities|FlowControl|Delay 0.9)
            (Audio|SpawnSoundatLocation (Variables|Default|GetSound) (Transformation|GetActorLocation (Game|GetPlayerCharacter 0)) "0, 0, 0" 1.0 1.0 0.0 0 0)
            (Default|PickUp (.AsBP%20FP (Utilities|Casting|CastToBP_FP (Game|GetPlayerCharacter 0)))))))
      (:Finished
        (Rendering|SetActorHiddenInGame true)))))

(event EventTick
  (params (DeltaSeconds :type Float%20%28single-precision%29)))

(fn ConstructionScript)